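; Bp_final is a goal trigger actor that ends the game once the player has collected enough items.
; Its Collectitem event increments the collected count and plays a pickup sound.
; When BP_ThirdPersonCharacter overlaps the Sphere, FinalCheck compares that count to the required maximum.
; If reached, a DoOnce fires Final, which shows the Wp_end widget and destroys the character.
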(event `Collectitem`
  (`/Engine/EditorBlueprintResources/StandardMacros.IncrementInt` (`self.CurrentItemsCollected`)
    (:`  `
      (`GameplayStatics.PlaySound2D` "/Game/Bp/collect-points-190037.collect-points-190037" 1.0 1.0 0.0 null null))))

(event `FinalCheck`
  (if (>= (`self.CurrentItemsCollected`) (`self.Maxitemscollecatble`))
    (`/Engine/EditorBlueprintResources/StandardMacros.DoOnce` false
      (:`Completed`
        (`self.Final`)))))

(event `self.Sphere.OnComponentBeginOverlap`
  (params (OverlappedComponent :type "PrimitiveComponent Object Reference") (OtherActor :type "Actor Object Reference") (OtherComp :type "PrimitiveComponent Object Reference") (OtherBodyIndex :type Integer) (bFromSweep :type Boolean) (SweepResult :type "HitResult Structure (by ref)"))
  (bind _asbp_third_person_character (cast `/Game/ThirdPerson/Blueprints/BP_ThirdPersonCharacter` OtherActor))
  (`self.FinalCheck`))

(event `Final`
  (bind _returnvalue (`|CreateWidget` "/Game/Bp/wp_end.wp_end_C"))
  (`UserWidget.AddToViewport` _returnvalue 0)
  (`self.K2_DestroyActor` (stale `self.Sphere.OnComponentBeginOverlap` _asbp_third_person_character)))

(fn `UserConstructionScript`)