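; Collectible item pickup that reacts when BP_ThirdPersonCharacter overlaps its Sphere component.
; On overlap it finds the Bp_final actor, calls its Collectitem, destroys itself and adds a white-tinted Items widget to the viewport.
; Disconnected leftover nodes for a tinted Items widget and a FakeItems widget with debug text never run.
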(event `self.Sphere.OnComponentBeginOverlap`
  (params (OverlappedComponent :type "PrimitiveComponent Object Reference") (OtherActor :type "Actor Object Reference") (OtherComp :type "PrimitiveComponent Object Reference") (OtherBodyIndex :type Integer) (bFromSweep :type Boolean) (SweepResult :type "HitResult Structure (by ref)"))
  (cast `/Game/ThirdPerson/Blueprints/BP_ThirdPersonCharacter` OtherActor)
  (bind _returnvalue (`GameplayStatics.GetActorOfClass` "/Game/Bp/Bp_final.Bp_final_C"))
  (`/Game/Bp/Bp_final.Collectitem` _returnvalue)
  (`self.K2_DestroyActor`)
  (bind _returnvalue_2 (`|CreateWidget` "/Game/ui/Items.Items_C"))
  (`UserWidget.SetColorAndOpacity` _returnvalue_2 (struct :`R` 1.0 :`G` 1.0 :`B` 1.0 :`A` 1.0))
  (`UserWidget.AddToViewport` _returnvalue_2 0))

(fn `UserConstructionScript`)