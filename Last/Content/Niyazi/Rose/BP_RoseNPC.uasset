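; BP_RoseNPC is the Rose NPC, which shows dialogue text one entry at a time.
; Each Talk event increments TalkIndex and writes that Dialouge array entry into a WBP_Dialouge widget, created and added to the viewport when no valid one exists.
; Once the index exceeds the array length, Talk removes the widget from its parent; the graph never resets the index.
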(event `/Game/Niyazi/Rose/BPI_Dialouge.Talk`
  (`/Engine/EditorBlueprintResources/StandardMacros.IncrementInt` (`self.TalkIndex`)
    (:`  `
      (if (<= (`self.TalkIndex`) (`KismetArrayLibrary.Array_Length` (`self.Dialouge`)))
        (`self.UI`
          (:`then`
            _)
          (:`else`
            (bind _returnvalue (`|CreateWidget` "/Game/Niyazi/Rose/WBP_Dialouge.WBP_Dialouge_C" (`GameplayStatics.GetPlayerController` 0)))
            (bind _output_get (set `self.UI` _returnvalue))
            (`UserWidget.AddToViewport` _output_get 0)))
        (`EditableTextBox.SetText` (`/Game/Niyazi/Rose/WBP_Dialouge.TalkText` (`self.UI`)) (`KismetTextLibrary.Conv_StringToText` (`|GetArrayItem` (`self.Dialouge`) (`self.TalkIndex`))))
        (else
          (`Widget.RemoveFromParent` (`self.UI`)))))))

(fn `UserConstructionScript`)